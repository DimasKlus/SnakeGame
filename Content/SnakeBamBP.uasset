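; SnakeBamBP is a deadly obstacle in a snake game that ends the run when a snake element touches it.
; On overlap with a SnakeElemBP it spawns a Niagara effect, plays a crash sound, destroys that element and, after a short delay, opens the GameOver level.
; The construction script gives its static mesh a random material from the shell material array for visual variety.
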(event EventBeginPlay)

(event Collision|EventActorBeginOverlap
  (params (OtherActor :type Actor%20Object%20Reference))
  (bind _assnake_elem_bp (Utilities|Casting|CastToSnakeElemBP OtherActor))
  (Utilities|IsValid _assnake_elem_bp
    (:Is%20Valid
      (Niagara|SpawnSystematLocation "/Game/sA_Megapack_v1/sA_Projectilevfx/Vfx/Fx/Niagara_Systems/NS_Muzzle_6.NS_Muzzle_6" "0, 0, 0")
      (Audio|PlaySound2D "/Game/material-zvukovoy-effekt-stolknoveniya-razdavit-39619.material-zvukovoy-effekt-stolknoveniya-razdavit-39619" 1.0 1.0 0.0 0 0)
      (Actor|DestroyActor _assnake_elem_bp)
      (Utilities|FlowControl|Delay 3.0)
      (Game|OpenLevel(byObjectReference) "/Game/GameOver.GameOver"))))

(fn ConstructionScript
  (Rendering|Material|SetMaterial (Variables|Default|GetStaticMesh) 0 (Utilities|Array|Get(acopy) (Variables|Default|GetShellMaterialArray) (Math|Random|RandomIntegerinRange 0 2))))